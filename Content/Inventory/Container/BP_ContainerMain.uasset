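; BP_ContainerMain is an interactable container actor that stores items in an InventorySystem component.
; Interacting with it pushes its content, size and self-reference to the interacting character's HUDPlayer, which then refreshes its container view.
; Add and remove events modify the inventory, then repeat that HUD update for the originating character.
; LookAt returns interaction text from the data table row referenced by NameId.
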(event `/Game/Inventory/Container/I_ContainerCommunication.AddToContainer`
  (params (Name :type Name) (Quantity :type Integer) (OriginCharacter :type "/Game/FirstPersonBP/Blueprints/FirstPersonCharacter Object Reference"))
  (`/Game/Inventory/InventorySystem.AddToInventory` (`self.InventorySystem`) Name Quantity)
  (`self.UpdateContainerInHud` OriginCharacter))

(event `/Game/Inventory/Container/I_ContainerCommunication.RemoveFromContainer`
  (params (Index :type Integer) (Quantity :type Integer) (OriginCharacter :type "/Game/FirstPersonBP/Blueprints/FirstPersonCharacter Object Reference"))
  (`/Game/Inventory/InventorySystem.RemoveFromInventory` (`self.InventorySystem`) Index Quantity)
  (`self.UpdateContainerInHud` OriginCharacter))

(fn `InteractWith`
  (params (OriginCharacter :type "/Game/FirstPersonBP/Blueprints/FirstPersonCharacter Object Reference"))
  (returns (IsContainer :type Boolean))
  (`self.UpdateContainerInHud` OriginCharacter)
  (return true))

(fn `LookAt`
  (returns (PickUpMessage :type Text))
  (bind (_nameid_datatable _nameid_rowname) (break `DataTableRowHandle` (`self.NameId`)))
  (bind _returnvalue (`|GetDataTableRow` _nameid_datatable _nameid_rowname)
    (:`then`
      (return (`.InteractionText_10_B3A50A6F4EBF6D83171A979F0264AA16` (break `/Game/Inventory/ContainerStruct` _returnvalue))))))

(fn `UpdateContainerInHud`
  (params (Origin :type "/Game/FirstPersonBP/Blueprints/FirstPersonCharacter Object Reference"))
  (bind _hud_player (`/Game/FirstPersonBP/Blueprints/FirstPersonCharacter.HUD_Player` Origin))
  (set `/Game/HUD/UMG/WBP_HUD_Player.Content_Container` (`/Game/Inventory/InventorySystem.Content` (`self.InventorySystem`)) _hud_player)
  (set `/Game/HUD/UMG/WBP_HUD_Player.ContainerSize` (`/Game/Inventory/InventorySystem.InventorySize` (`self.InventorySystem`)) _hud_player)
  (set `/Game/HUD/UMG/WBP_HUD_Player.CurrentContainer` self _hud_player)
  (`/Game/HUD/UMG/WBP_HUD_Player.Update Container` _hud_player))

(fn `UserConstructionScript`)
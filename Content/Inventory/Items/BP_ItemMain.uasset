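; World pickup actor for inventory items, defined by a data table row handle and a quantity set through InitItem.
; InteractWith adds the item to the interacting character's InventorySystem, keeps any remainder, and destroys the actor at zero.
; For rows flagged as ammo, it also calls the character's AmmoInInventory.
; LookAt returns the row's pickup text.
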(event `/Game/Inventory/I_ItemCommunication.InitItem`
  (params (ItemID :type "DataTableRowHandle Structure") (Quantity :type Integer))
  (set `self.ItemId` ItemID)
  (set `self.Quantity` Quantity))

(fn `InteractWith`
  (params (OriginCharacter :type "/Game/FirstPersonBP/Blueprints/FirstPersonCharacter Object Reference"))
  (returns (IsContainer :type Boolean))
  (bind (_itemid_datatable _itemid_rowname) (break `DataTableRowHandle` (`self.ItemId`)))
  (bind (_success _quantityremaining) (`/Game/Inventory/InventorySystem.AddToInventory` (`/Game/FirstPersonBP/Blueprints/FirstPersonCharacter.InventorySystem` OriginCharacter) _itemid_rowname (`self.Quantity`)))
  (if _success
    (set `self.Quantity` _quantityremaining)
    (bind _returnvalue (`|GetDataTableRow` "/Game/Inventory/ItemDataTable.ItemDataTable" _itemid_rowname)
      (:`then`
        (if (`.IsAmmo_35_4005F4E54317730E0C12FB84EFC4D14E` (break `/Game/Inventory/ItemStruct` _returnvalue))
          (`/Game/FirstPersonBP/Blueprints/FirstPersonCharacter.AmmoInInventory` OriginCharacter)
          (if (== (`self.Quantity`) 0)
            (`self.K2_DestroyActor`)
            (return false))
          (elif (== (`self.Quantity`) 0)
            (`self.K2_DestroyActor`)
            (return false)))))))

(fn `LookAt`
  (returns (PickUpMessage :type Text))
  (bind (_itemid_datatable _itemid_rowname) (break `DataTableRowHandle` (`self.ItemId`)))
  (bind _returnvalue (`|GetDataTableRow` _itemid_datatable _itemid_rowname)
    (:`then`
      (return (`.PickUpText_9_8AEC9A214A64FB3A3ED8B9B7C114A73E` (break `/Game/Inventory/ItemStruct` _returnvalue))))))

(fn `UserConstructionScript`)